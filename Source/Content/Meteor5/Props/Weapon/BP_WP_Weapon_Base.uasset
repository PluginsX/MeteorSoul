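; Base weapon actor that bobs until a XingHun character picks it up into a two-slot array and hand socket.
; While its owner attacks, Box overlaps on enemy Meteor_AI spawn random GameMode blood effects and decals, then send the hit direction to OnAcceptAttack.
; SpawnSkill maps skill section names to events that set owner particles, apply movement impulses or switch root motion to montage-only.
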(event `self.ReceiveBeginPlay`
  ;[1 1 1] 游戏开始时武器需要获取游戏模式的引用
  (bind _asmeteor_game_mode (cast `/Game/Meteor5/Class/MeteorGameMode` (`GameplayStatics.GetGameMode`)))
  (set `self.GameMode` _asmeteor_game_mode))

(event `self.Box.OnComponentBeginOverlap`
  (params (OverlappedComponent :type "PrimitiveComponent Object Reference") (OtherActor :type "Actor Object Reference") (OtherComp :type "PrimitiveComponent Object Reference") (OtherBodyIndex :type Integer) (bFromSweep :type Boolean) (SweepResult :type "HitResult Structure (by ref)"))
  (bind _returnvalue (`self.K2_GetActorLocation`))
  (bind _fx_bloodparticlearray (`/Game/Meteor5/Class/MeteorGameMode.FX_BloodParticleArray` (`self.GameMode`)))
  (bind _fx_decalarray (`/Game/Meteor5/Class/MeteorGameMode.FX_DecalArray` (`self.GameMode`)))
  (`|ExecutionSequence`
    (:`then_0`
      ;[1 1 1] 拾取检测
      (`/Engine/EditorBlueprintResources/StandardMacros.DoOnce` false
        (:`Completed`
          (bind _asxing_hun (cast `/Game/Meteor5/Class/Charactor/XingHun` OtherActor))
          (bind _weaponarray (`/Game/Meteor5/Class/Charactor/XingHun.WeaponArray` _asxing_hun))
          (bind _returnvalue_2 (`KismetArrayLibrary.Array_Length` _weaponarray))
          (if (< _returnvalue_2 2)
            (if (== _returnvalue_2 0)
              (`KismetArrayLibrary.Array_Add` _weaponarray self)
              (set `self.WeaponOwner` _asxing_hun)
              (`self.K2_AttachToComponent` (`Character.Mesh` _asxing_hun) "d_wpnRP" "SnapToTarget" "SnapToTarget" "SnapToTarget" :!label _label)
              (set `self.OnHand` true)
              (else
                (`KismetArrayLibrary.Array_Add` _weaponarray self)
                (bind _output (`|GetArrayItem` _weaponarray))
                (if (`KismetSystemLibrary.IsValid` _output)
                  (`SceneComponent.SetVisibility` (`/Game/Meteor5/Props/Weapon/BP_WP_Weapon_Base.SkeletalMesh` _output) false false)
                  (goto _label))))))))
    (:`then_1`
      ;[1 0.04947 0] 击中事件
      (if (`.STATE_Attack_22_20F81B4E4031A02BD63290B4DA9AECE3` (break `/Game/Meteor5/Struct/STRUCT_Charactor_State` (`/Game/Meteor5/Class/Charactor/XingHun.State` (`self.WeaponOwner`))))
        (`|ExecutionSequence`
          (:`then_0`
            ;[1 1 1] 击中敌人
            (bind _asmeteor_ai (cast `/Game/Meteor5/AI/Meteor_AI` OtherActor))
            (if (`self.ActorHasTag` _asmeteor_ai "AI_Enemy")
              (`|ExecutionSequence`
                (:`then_0`
                  (bind _returnvalue_3 (`self.K2_GetActorLocation` _asmeteor_ai))
                  ;[1 1 1] 流血粒子特效
                  (`GameplayStatics.SpawnEmitterAtLocation` (`|GetArrayItem` _fx_bloodparticlearray (`KismetMathLibrary.RandomIntegerInRange` 0 (- (`KismetArrayLibrary.Array_Length` _fx_bloodparticlearray) 1))) _returnvalue_3)
                  (`|ExecutionSequence`
                    (:`then_0`
                      ;[0.2917 0.6686 1] DEBUG
                      (`KismetSystemLibrary.DrawDebugArrow` (+ _returnvalue (* (`KismetMathLibrary.Normal` (- _returnvalue _returnvalue_3)) 100)) _returnvalue 100.0 (struct :`R` 1.0 :`G` 0.053326 :`A` 1.0) 1.0 10.0))
                    (:`then_1`
                      ;[1 1 1] 根据重叠位置与 角色 位置 计算出 攻击方向，用于动画\触发被击角色的受击事件，传入受击方位，和伤害量
                      (bind _relativeangle (`/Game/Meteor5/Function/PublicFunction.CalcRelativAngleByRotator` (`KismetMathLibrary.Normal` (- (`self.K2_GetActorLocation`) _returnvalue_3)) (`self.K2_GetActorRotation` _asmeteor_ai)))
                      (bind _directiontype (`self.ClacAttackDirectionFromAngle` _relativeangle))
                      (`/Game/Meteor5/AI/Meteor_AI.OnAcceptAttack` _asmeteor_ai _directiontype))))
                (:`then_1`
                  ;[1 1 1] 生成贴画材质
                  (`/Engine/EditorBlueprintResources/StandardMacros.DoOnce` false :!label _label_2
                    (:`Completed`
                      (`GameplayStatics.SpawnDecalAtLocation` (`|GetArrayItem` _fx_decalarray (`KismetMathLibrary.RandomIntegerInRange` 0 (- (`KismetArrayLibrary.Array_Length` _fx_decalarray) 1))) (300.0 100.0 100.0) (`KismetMathLibrary.MakeVector` (.x _returnvalue_3) (.y _returnvalue_3) (.z _returnvalue_3)) (`KismetMathLibrary.MakeRotator` 0.0 -90.0 (`KismetMathLibrary.Conv_IntToDouble` (`KismetMathLibrary.RandomIntegerInRange` 0 360))) 2.0)
                      (`KismetSystemLibrary.Delay` 2.0) ; 贴画生命周期为2，一个消失一个才出现
                      (goto _label_2 :!via `Reset`))))))))))))

(event `self.ReceiveTick`
  (params (DeltaSeconds :type "Float (single-precision)"))
  (bind _defaultsceneroot (`self.DefaultSceneRoot`))
  (`|ExecutionSequence`
    (:`then_0`
      ;[1 1 1] 被拾取之前，上下浮动
      (if (not (`self.OnHand`))
        (bind _output_get (set `self.Zadd` (+ 1.0 (`self.Zadd`))))
        (bind _returnvalue (`KismetMathLibrary.DegCos` _output_get))
        (`SceneComponent.K2_AddWorldOffset` _defaultsceneroot (`KismetMathLibrary.MakeVector` 0.0 0.0 (* _returnvalue 0.1)) false false)
        (`SceneComponent.K2_AddWorldRotation` _defaultsceneroot (`KismetMathLibrary.MakeRotator` 0.0 0.0 _returnvalue) false false)))))

(event `self.Box.OnComponentEndOverlap`
  (params (OverlappedComponent :type "PrimitiveComponent Object Reference") (OtherActor :type "Actor Object Reference") (OtherComp :type "PrimitiveComponent Object Reference") (OtherBodyIndex :type Integer)))

(event `Skill_FX_G_2110`
  ;[1 1 1] 匕首特效_2110
  (`ParticleSystemComponent.SetTemplate` (`/Game/Meteor5/Class/Charactor/XingHun.Particle` (`self.WeaponOwner`)) "/Game/Meteor5/FX/SkillEffects/AdvancedMagicFX14/Particles/P_ky_lightning2.P_ky_lightning2")
  (`KismetSystemLibrary.Delay` 0.8)
  (`GameplayStatics.SpawnEmitterAtLocation` "/Game/Meteor5/FX/SkillEffects/AdvancedMagicFX14/Particles/P_ky_lightning1.P_ky_lightning1" (`self.K2_GetActorLocation`) (`KismetMathLibrary.MakeRotator` (.roll (`self.K2_GetActorRotation` (`self.WeaponOwner`))) (.pitch (`self.K2_GetActorRotation` (`self.WeaponOwner`))) (+ (.yaw (`self.K2_GetActorRotation` (`self.WeaponOwner`))) 180.0)) (0.5 0.5 0.5)))

(event `Skill_FX_G_110`
  ;[1 1 1] 匕首特效_110
  (`KismetSystemLibrary.Delay` 0.7)
  (`ParticleSystemComponent.SetTemplate` (`/Game/Meteor5/Class/Charactor/XingHun.Particle` (`self.WeaponOwner`)) "/Game/Meteor5/FX/SkillEffects/AdvancedMagicFX14/Particles/P_ky_fireVortex3.P_ky_fireVortex3"))

(event `Skill_FX_A_20`
  ;[1 1 1] 匕首特效_20
  (`KismetSystemLibrary.Delay` 0.2)
  (`ParticleSystemComponent.SetTemplate` (`/Game/Meteor5/Class/Charactor/XingHun.Particle` (`self.WeaponOwner`)) "/Game/Meteor5/FX/SkillEffects/AdvancedMagicFX14/Particles/P_ky_flareRise.P_ky_flareRise"))

(event `Skill_FX_A_120`
  ;[1 1 1] A_120
  (`KismetSystemLibrary.Delay` 0.2)
  (`ParticleSystemComponent.SetTemplate` (`/Game/Meteor5/Class/Charactor/XingHun.Particle` (`self.WeaponOwner`)) "/Game/Meteor5/FX/SkillEffects/AdvancedMagicFX14/Particles/P_ky_shockwave.P_ky_shockwave"))

(event `Skill_Motion_A_20`
  ;[1 1 1] DownFoce
  (`CharacterMovementComponent.AddImpulse` (`Character.CharacterMovement` (`self.WeaponOwner`)) (0.0 0.0 -500.0) true))

(event `Skill_Motion_A_120`
  (bind _weaponowner (`self.WeaponOwner`))
  (`|ExecutionSequence`
    (:`then_0`
      ;[1 1 1] DownFoce
      (`CharacterMovementComponent.AddImpulse` (`Character.CharacterMovement` _weaponowner) (* (+ (`KismetMathLibrary.Normal` (`SceneComponent.GetForwardVector` (`Actor.RootComponent` _weaponowner))) (0.0 0.0 -0.6)) 800) true))
    (:`then_1`
      ;[1 1 1] RootMotionMoldChange
      (`AnimInstance.SetRootMotionMode` (`SkeletalMeshComponent.GetAnimInstance` (`Character.Mesh` (`self.WeaponOwner`))) "RootMotionFromMontagesOnly" :!label _label))))

(event `Skill_Motion_A_0`
  (bind _weaponowner (`self.WeaponOwner`))
  ;[1 1 1] UpFoce
  (if (< (.z (`self.GetVelocity` _weaponowner)) 0.0) :!label _label_2
    (`CharacterMovementComponent.AddImpulse` (`Character.CharacterMovement` _weaponowner) (`KismetMathLibrary.MakeVector` 0.0 0.0 600.0) true)))

(event `Skill_Motion_A_0_0`
  (goto _label_2))

(event `Skill_Motion_A_0_0_0`
  (goto _label_2))

(event `Skill_Motion_G_110`
  (`|ExecutionSequence`
    (:`then_0`
      (goto _label))
    (:`then_1`
      (`KismetSystemLibrary.Delay` 0.8)
      ;[1 1 1] UpFoce
      (`CharacterMovementComponent.AddImpulse` (`Character.CharacterMovement` (`self.WeaponOwner`)) (0.0 0.0 600.0) true))))

(event `Skill_Motion_G_10`
  (goto _label))

(event `Skill_Motion_G_30`
  (goto _label))

(event `Skill_Motion_G_40`
  (goto _label))

(event `Skill_Motion_G_210`
  (goto _label))

(event `Skill_Motion_G_2110`
  (goto _label))

(event `Skill_Motion_G_11`
  ;[1 1 1] 闪避
  (goto _label))

(event `Skill_Motion_G_22`
  ;[1 1 1] 闪避
  (goto _label))

(event `Skill_Motion_G_33`
  ;[1 1 1] 闪避
  (goto _label))

(event `Skill_Motion_G_44`
  ;[1 1 1] 闪避
  (goto _label))

(fn `ClacAttackDirectionFromAngle`
  (params (NewParam :type "Rotator Structure"))
  (returns (DirectionType :type Integer))
  (bind _yaw (.yaw NewParam))
  ;[1 1 1] ForwardAttack
  (if (and (> _yaw -45.0) (< _yaw 45.0))
    (return 1)
    (else
      ;[1 1 1] BackAttack
      (if (and (<= _yaw -135.0) (>= _yaw 135.0))
        (return 2)
        (else
          ;[1 1 1] LeftAttack
          (if (and (> _yaw -135.0) (<= _yaw -45.0))
            (return 3)
            (else
              ;[1 1 1] RightAttack
              (if (and (>= _yaw 45.0) (< _yaw 135.0))
                (return 4)))))))))

(fn `SpawnSkill`
  (params (SkillSectionName :type String))
  ;[1 1 1] 根据获得的技能编号，执行技能的函数
  (if (`KismetStringLibrary.EqualEqual_StrStr` SkillSectionName "G_2110")
    ;[1 1 1] FX
    (`self.Skill_FX_G_2110`)
    ;[1 1 1] Motion
    (`self.Skill_Motion_G_2110`)
    (elif (`KismetStringLibrary.EqualEqual_StrStr` SkillSectionName "A_120")
      (`self.Skill_FX_A_120`)
      (`self.Skill_Motion_A_120`)
      (elif (`KismetStringLibrary.EqualEqual_StrStr` SkillSectionName "A_20")
        (`self.Skill_FX_A_20`)
        (`self.Skill_Motion_A_20`)
        (elif (`KismetStringLibrary.EqualEqual_StrStr` SkillSectionName "G_110")
          (`self.Skill_FX_G_110`)
          (`self.Skill_Motion_G_110`)
          (elif (`KismetStringLibrary.EqualEqual_StrStr` SkillSectionName "A_0")
            (`self.Skill_Motion_A_0`)
            (elif (`KismetStringLibrary.EqualEqual_StrStr` SkillSectionName "A_0_0")
              (`self.Skill_Motion_A_0_0`)
              (elif (`KismetStringLibrary.EqualEqual_StrStr` SkillSectionName "A_0_0_0")
                (`self.Skill_Motion_A_0_0_0`)
                (elif (`KismetStringLibrary.EqualEqual_StrStr` SkillSectionName "G_10")
                  (`self.Skill_Motion_G_10`)
                  (elif (`KismetStringLibrary.EqualEqual_StrStr` SkillSectionName "G_30")
                    (`self.Skill_Motion_G_30`)
                    (elif (`KismetStringLibrary.EqualEqual_StrStr` SkillSectionName "G_40")
                      (`self.Skill_Motion_G_40`)
                      (elif (`KismetStringLibrary.EqualEqual_StrStr` SkillSectionName "G_210")
                        (`self.Skill_Motion_G_210`)
                        (elif (`KismetStringLibrary.EqualEqual_StrStr` SkillSectionName "G_11")
                          (`self.Skill_Motion_G_11`)
                          (elif (`KismetStringLibrary.EqualEqual_StrStr` SkillSectionName "G_22")
                            (`self.Skill_Motion_G_22`)
                            (elif (`KismetStringLibrary.EqualEqual_StrStr` SkillSectionName "G_33")
                              (`self.Skill_Motion_G_33`)
                              (elif (`KismetStringLibrary.EqualEqual_StrStr` SkillSectionName "G_44")
                                (`self.Skill_Motion_G_44`)))))))))))))))))

(fn `UserConstructionScript`)